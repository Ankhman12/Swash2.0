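; Gameplay ability for Jack's melee attack B, which starts a melee attack on the owning BP_SwashTemplateCharacter and plays a montage while blocking cancellation.
; A one-shot Melee.Hit event listener applies GE_Damage to the event's targets and records the hit.
; Montage completion tries a combo reset, re-enables cancellation and ends the ability.
; On end, it breaks the combo if nothing was hit, ends the melee attack and cleans up both async tasks.
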(event `self.K2_ActivateAbility`
  (`self.SetCanBeCanceled` false)
  (bind _asbp_swash_template_character (cast `/Game/MitchellsStuff/BP_SwashTemplateCharacter` (`.OwnerActor` (break `GameplayAbilityActorInfo` (`self.GetActorInfo`))))
    (:`then`
      (`/Game/MitchellsStuff/BP_SwashTemplateCharacter.StartMeleeAttack` _asbp_swash_template_character)
      (bind _asynctaskproxy (`AbilityTask_PlayMontageAndWait.CreatePlayMontageAndWaitProxy` "None" (`self.Montage`))
        (:`then`
          (set `self.Async Attack Task` _asynctaskproxy)
          (bind (_asynctaskproxy_2 _payload) (`AbilityTask_WaitGameplayEvent.WaitGameplayEvent` (struct :`TagName` "Melee.Hit") null true)
            (:`then`
              (set `self.Async Hit Task` _asynctaskproxy_2))
            (:`EventReceived`
              (`self.BP_ApplyGameplayEffectToTarget` (`.TargetData` (break `GameplayEventData` _payload)) "/Game/MitchellsStuff/GE_Damage.GE_Damage_C")
              (set `self.Hit?` true))))
        (:`OnCompleted`
          (`/Game/MitchellsStuff/BP_SwashTemplateCharacter.TryResetCombo` _asbp_swash_template_character)
          (`KismetSystemLibrary.PrintString` "Hello" true true (struct :`R` 1.0 :`B` 0.834041 :`A` 1.0))
          (`self.SetCanBeCanceled` true)
          (`self.K2_EndAbility`))))
    (:`CastFailed`
      (`self.K2_EndAbility`))))

(event `self.K2_OnEndAbility`
  (params (bWasCancelled :type Boolean))
  (bind _async_hit_task (`self.Async Hit Task`))
  (bind _async_attack_task (`self.Async Attack Task`))
  (if (not (`self.Hit?`))
    (`/Game/MitchellsStuff/BP_SwashTemplateCharacter.EndCombo` (stale `self.K2_ActivateAbility` _asbp_swash_template_character)))
  (`/Game/MitchellsStuff/BP_SwashTemplateCharacter.EndMeleeAttack` (stale `self.K2_ActivateAbility` _asbp_swash_template_character))
  (`|ExecutionSequence`
    (:`then_0`
      (`/Engine/EditorBlueprintResources/StandardMacros.IsValid` _async_hit_task
        (:`Is Valid`
          (`GameplayTask.EndTask` _async_hit_task))))
    (:`then_1`
      (`/Engine/EditorBlueprintResources/StandardMacros.IsValid` _async_attack_task
        (:`Is Valid`
          (`GameplayTask.EndTask` _async_attack_task))))))