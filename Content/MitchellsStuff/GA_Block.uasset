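; GA_Block is a gameplay ability that puts the swashbuckler character into a blocking state.
; On activation it stops movement, ignores move input and applies the GE_Blocking effect, then waits for a Melee.Block.End gameplay event.
; That event, or cancellation, restores move input and removes effects granting State.Blocking, and ending the ability also ends the wait task.
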(event `self.K2_ActivateAbility`
  (bind _asbp_swash_template_character (cast `/Game/MitchellsStuff/BP_SwashTemplateCharacter` (`.OwnerActor` (break `GameplayAbilityActorInfo` (`self.GetActorInfo`)))))
  (`MovementComponent.StopMovementImmediately` (`Character.CharacterMovement` _asbp_swash_template_character))
  (`Controller.SetIgnoreMoveInput` (`Pawn.GetController` _asbp_swash_template_character) true)
  (`AbilitySystemComponent.BP_ApplyGameplayEffectToSelf` :`self` (`SwashCharacter.AbilitySystemComponent` _asbp_swash_template_character) :`GameplayEffectClass` "/Game/MitchellsStuff/GE_Blocking.GE_Blocking_C")
  ;[1 1 1] Wait to end block
  (bind _asynctaskproxy (`AbilityTask_WaitGameplayEvent.WaitGameplayEvent` (struct :`TagName` "Melee.Block.End") null true)
    (:`then`
      (set `self.BlockingTask` _asynctaskproxy))
    (:`EventReceived`
      (`Controller.ResetIgnoreMoveInput` (`Pawn.GetController` _asbp_swash_template_character))
      (`AbilitySystemComponent.RemoveActiveEffectsWithGrantedTags` (`SwashCharacter.AbilitySystemComponent` _asbp_swash_template_character) (struct :`GameplayTags` (struct :`(TagName` "State.Blocking"))))
      (`self.K2_EndAbility`))))

(event `self.K2_OnEndAbility`
  (params (bWasCancelled :type Boolean))
  (bind _blockingtask (`self.BlockingTask`))
  (`|ExecutionSequence`
    (:`then_0`
      (if bWasCancelled
        (`Controller.ResetIgnoreMoveInput` (`Pawn.GetController` (stale `self.K2_ActivateAbility` _asbp_swash_template_character)))
        (`AbilitySystemComponent.RemoveActiveEffectsWithGrantedTags` (`SwashCharacter.AbilitySystemComponent` (stale `self.K2_ActivateAbility` _asbp_swash_template_character)) (struct :`GameplayTags` (struct :`(TagName` "State.Blocking"))))))
    (:`then_1`
      (`/Engine/EditorBlueprintResources/StandardMacros.IsValid` _blockingtask
        (:`Is Valid`
          (`GameplayTask.EndTask` _blockingtask))))))