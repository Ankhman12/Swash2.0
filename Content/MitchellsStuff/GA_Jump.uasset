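; Gameplay Ability that makes the BP_SwashTemplateCharacter owner jump.
; On activation it starts the jump, flags the jump as held and ends any block.
; A WaitGameplayEvent task then listens once for Movement.Jump.End on the character, which stops the jump, clears the held flag and ends the ability.
; The task is stored in JumpTask, but OnEndAbility is empty, so cleanup happens only when that event arrives.
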(event `self.K2_ActivateAbility`
  (bind _asbp_swash_template_character (cast `/Game/MitchellsStuff/BP_SwashTemplateCharacter` (`.OwnerActor` (break `GameplayAbilityActorInfo` (`self.GetActorInfo`)))))
  (`Character.Jump` _asbp_swash_template_character)
  (set `SwashCharacter.IsHoldingJump` true _asbp_swash_template_character)
  (`SwashCharacter.EndBlock` _asbp_swash_template_character)
  (bind _asynctaskproxy (`AbilityTask_WaitGameplayEvent.WaitGameplayEvent` (struct :`TagName` "Movement.Jump.End") _asbp_swash_template_character true)
    (:`then`
      (set `self.JumpTask` _asynctaskproxy))
    (:`EventReceived`
      (`Character.StopJumping` _asbp_swash_template_character)
      (set `SwashCharacter.IsHoldingJump` false _asbp_swash_template_character)
      (`self.K2_EndAbility`))))

(event `self.K2_OnEndAbility`
  (params (bWasCancelled :type Boolean)))